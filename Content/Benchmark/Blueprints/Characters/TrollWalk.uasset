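; TrollWalk is a benchmark troll pawn that supplies walk destinations to its AI controller.
; On BeginPlay it casts its controller to TrollAI and copies its four destination variables into the controller's matching variables, printing a message if the cast fails.
; It contains no movement logic itself, and its construction script is empty.
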(event `self.ReceiveBeginPlay`
  (bind _astroll_ai (cast `/Game/Benchmark/Blueprints/Characters/TrollAI` (`self.GetController`))
    (:`then`
      (set `/Game/Benchmark/Blueprints/Characters/TrollAI.Dest1` (`self.Dest1`) _astroll_ai)
      (set `/Game/Benchmark/Blueprints/Characters/TrollAI.Dest2` (`self.Dest2`) _astroll_ai)
      (set `/Game/Benchmark/Blueprints/Characters/TrollAI.Dest3` (`self.Dest3`) _astroll_ai)
      (set `/Game/Benchmark/Blueprints/Characters/TrollAI.Dest4` (`self.Dest4`) _astroll_ai))
    (:`CastFailed`
      (`KismetSystemLibrary.PrintString` "failed to cast"))))

(fn `UserConstructionScript`)