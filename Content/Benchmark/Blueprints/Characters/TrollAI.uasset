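; Troll AI Blueprint for the Benchmark content that walks a looping patrol through four destination actors.
; BeginPlay starts the route at once if DelayStart is set, otherwise it waits briefly and sets the flag first.
; Chained AIMoveTo nodes visit Dest1 to Dest4 in order, and the last finish wires back to the first move.
; Any failed request prints a navigation error and ends the patrol without retrying.
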(event `self.ReceiveBeginPlay`
  (if (`self.bDelayStart`) :!label _label
    (`AITask_MoveTo.AIMoveTo` null (0.0 0.0 0.0) (`self.Dest1`) :!label _label_2
      (:`OnRequestFailed`
        _)
      (:`OnMoveFinished`
        (`AITask_MoveTo.AIMoveTo` null (0.0 0.0 0.0) (`self.Dest2`)
          (:`OnRequestFailed`
            _)
          (:`OnMoveFinished`
            (`AITask_MoveTo.AIMoveTo` null (0.0 0.0 0.0) (`self.Dest3`)
              (:`OnRequestFailed`
                _)
              (:`OnMoveFinished`
                (`AITask_MoveTo.AIMoveTo` null (0.0 0.0 0.0) (`self.Dest4`)
                  (:`OnRequestFailed`
                    _)
                  (:`OnMoveFinished`
                    (goto _label_2)))))))))
    (`KismetSystemLibrary.PrintString` "failed navigating")
    (else
      (`KismetSystemLibrary.Delay` 2.0)
      (set `self.bDelayStart` true)
      (goto _label))))

(fn `UserConstructionScript`)